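; Destructible tower actor that breaks apart one of three variants (low, mid or high) when ConstructDestruction is called.
; It destroys the components of the other two variants, then lifts the chosen body, shield and platform and gives them dynamic material instances.
; Radius damage with impulse, stronger for higher variants, shatters those pieces.
; The three material instances are then handed to FadeOut.
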(event Collision|EventActorBeginOverlap
  (params (OtherActor :type Actor%20Object%20Reference)))

(event EventTick
  (params (DeltaSeconds :type Float%20%28single-precision%29)))

(event EventConstructDestruction
  (params (materialToApply :type Material%20Instance%20Object%20Reference) (lowMidHigh :type Integer))
  (bind _towerbodyhigh (Variables|Default|GetTowerBodyHigh))
  (bind _shieldhigh (Variables|Default|GetShieldHigh))
  (bind _platformhigh (Variables|Default|GetPlatformHigh))
  (bind _towerbodylow (Variables|Default|GetTowerBodyLow))
  (bind _shieldlow (Variables|Default|GetShieldLow))
  (bind _platformlow (Variables|Default|GetPlatformLow))
  (bind _towerbodymid (Variables|Default|GetTowerBodyMid))
  (bind _shieldmid (Variables|Default|GetShieldMid))
  (bind _platformmid (Variables|Default|GetPlatformMid))
  (bind _returnvalue (Transformation|GetWorldLocation _shieldmid))
  (bind _returnvalue_2 (Transformation|GetWorldLocation _shieldlow))
  (bind _returnvalue_3 (Transformation|GetWorldLocation _shieldhigh))
  (bind _returnvalue_4 (Rendering|Material|CreateDynamicMaterialInstance "/Game/Materials/Glow/Tower/Tower.Tower" "None" :!class /Script/Engine.KismetMaterialLibrary))
  (Variables|Default|SetInstanceTower _returnvalue_4)
  (bind _returnvalue_5 (Rendering|Material|CreateDynamicMaterialInstance "/Game/Materials/Glow/Tower/Tower1.Tower1" "None" :!class /Script/Engine.KismetMaterialLibrary))
  (Variables|Default|SetInstanceTower1 _returnvalue_5)
  (bind _returnvalue_6 (Rendering|Material|CreateDynamicMaterialInstance "/Game/Materials/Glow/Tower/Tower2.Tower2" "None" :!class /Script/Engine.KismetMaterialLibrary))
  (Variables|Default|SetInstanceTower2 _returnvalue_6)
  (switch int lowMidHigh
    (:1
      (Components|DestroyComponent (Variables|Default|GetTowerBodyMid))
      (Components|DestroyComponent (Variables|Default|GetTowerBodyHigh))
      (Components|DestroyComponent (Variables|Default|GetShieldMid))
      (Components|DestroyComponent (Variables|Default|GetPlatformHigh))
      (Components|DestroyComponent (Variables|Default|GetPlatformMid))
      (Components|DestroyComponent (Variables|Default|GetShieldHigh))
      (Transformation|AddLocalOffset _towerbodylow "0,0.000000,1500.000000" false true)
      (Rendering|Material|SetMaterial _towerbodylow 0 (Variables|Default|GetInstanceTower1))
      (Rendering|Material|SetMaterial _towerbodylow 1 (Variables|Default|GetInstanceTower1))
      (Rendering|Material|SetMaterial _towerbodylow 3 (Variables|Default|GetInstanceTower1))
      (Class|DestructibleComponent|ApplyRadiusDamage _towerbodylow 1e+03 _returnvalue_2 3e+03 5e+04 true)
      (Transformation|AddLocalOffset _shieldlow "0,0.000000,1500.000000" false true)
      (Rendering|Material|SetMaterial _shieldlow 0 (Variables|Default|GetInstanceTower))
      (Rendering|Material|SetMaterial _shieldlow 1 (Variables|Default|GetInstanceTower))
      (Rendering|Material|SetMaterial _shieldlow 3 (Variables|Default|GetInstanceTower))
      (Class|DestructibleComponent|ApplyRadiusDamage _shieldlow 1e+03 _returnvalue_2 3e+03 5e+04 true)
      (Transformation|AddLocalOffset _platformlow "0,0.000000,3000.000000" false true)
      (Rendering|Material|SetMaterial _platformlow 0 (Variables|Default|GetInstanceTower2))
      (Rendering|Material|SetMaterial _platformlow 1 (Variables|Default|GetInstanceTower2))
      (Rendering|Material|SetMaterial _platformlow 3 (Variables|Default|GetInstanceTower2))
      (Class|DestructibleComponent|ApplyRadiusDamage _platformlow 1e+03 (Transformation|GetWorldLocation _platformlow) 5e+02 2.5e+04 true))
    (:2
      (Components|DestroyComponent (Variables|Default|GetTowerBodyLow))
      (Components|DestroyComponent (Variables|Default|GetTowerBodyHigh))
      (Components|DestroyComponent (Variables|Default|GetShieldLow))
      (Components|DestroyComponent (Variables|Default|GetPlatformHigh))
      (Components|DestroyComponent (Variables|Default|GetPlatformLow))
      (Components|DestroyComponent (Variables|Default|GetShieldHigh))
      (Transformation|AddLocalOffset _towerbodymid "0,0.000000,1500.000000" false true)
      (Rendering|Material|SetMaterial _towerbodymid 0 (Variables|Default|GetInstanceTower1))
      (Rendering|Material|SetMaterial _towerbodymid 1 (Variables|Default|GetInstanceTower1))
      (Rendering|Material|SetMaterial _towerbodymid 3 (Variables|Default|GetInstanceTower1))
      (Class|DestructibleComponent|ApplyRadiusDamage _towerbodymid 1e+03 _returnvalue 3e+03 1e+05 true)
      (Transformation|AddLocalOffset _shieldmid "0,0.000000,1500.000000" false true)
      (Rendering|Material|SetMaterial _shieldmid 0 (Variables|Default|GetInstanceTower))
      (Rendering|Material|SetMaterial _shieldmid 1 (Variables|Default|GetInstanceTower))
      (Rendering|Material|SetMaterial _shieldmid 3 (Variables|Default|GetInstanceTower))
      (Class|DestructibleComponent|ApplyRadiusDamage _shieldmid 1e+03 _returnvalue 3e+03 1e+05 true)
      (Transformation|AddLocalOffset _platformmid "0,0.000000,3000.000000" false true)
      (Rendering|Material|SetMaterial _platformmid 0 (Variables|Default|GetInstanceTower2))
      (Rendering|Material|SetMaterial _platformmid 1 (Variables|Default|GetInstanceTower2))
      (Rendering|Material|SetMaterial _platformmid 3 (Variables|Default|GetInstanceTower2))
      (Class|DestructibleComponent|ApplyRadiusDamage _platformmid 1e+03 (Transformation|GetWorldLocation _platformmid) 5e+02 5e+04 true))
    (:3
      (Components|DestroyComponent (Variables|Default|GetTowerBodyMid))
      (Components|DestroyComponent (Variables|Default|GetShieldLow))
      (Components|DestroyComponent (Variables|Default|GetShieldMid))
      (Components|DestroyComponent (Variables|Default|GetPlatformLow))
      (Components|DestroyComponent (Variables|Default|GetPlatformMid))
      (Components|DestroyComponent (Variables|Default|GetTowerBodyLow))
      (Transformation|AddLocalOffset _towerbodyhigh "0,0.000000,1500.000000" false true)
      (Rendering|Material|SetMaterial _towerbodyhigh 0 (Variables|Default|GetInstanceTower1))
      (Rendering|Material|SetMaterial _towerbodyhigh 1 (Variables|Default|GetInstanceTower1))
      (Rendering|Material|SetMaterial _towerbodyhigh 3 (Variables|Default|GetInstanceTower1))
      (Class|DestructibleComponent|ApplyRadiusDamage _towerbodyhigh 1e+03 _returnvalue_3 3e+03 1.5e+05 true)
      (Transformation|AddLocalOffset _shieldhigh "0,0.000000,1500.000000" false true)
      (Rendering|Material|SetMaterial _shieldhigh 0 (Variables|Default|GetInstanceTower))
      (Rendering|Material|SetMaterial _shieldhigh 1 (Variables|Default|GetInstanceTower))
      (Rendering|Material|SetMaterial _shieldhigh 3 (Variables|Default|GetInstanceTower))
      (Class|DestructibleComponent|ApplyRadiusDamage _shieldhigh 1e+03 _returnvalue_3 3e+03 1.5e+05 true)
      (Transformation|AddLocalOffset _platformhigh "0,0.000000,3000.000000" false true)
      (Rendering|Material|SetMaterial _platformhigh 0 (Variables|Default|GetInstanceTower2))
      (Rendering|Material|SetMaterial _platformhigh 1 (Variables|Default|GetInstanceTower2))
      (Rendering|Material|SetMaterial _platformhigh 3 (Variables|Default|GetInstanceTower2))
      (Class|DestructibleComponent|ApplyRadiusDamage _platformhigh 1e+03 (Transformation|GetWorldLocation _platformhigh) 5e+02 7.5e+04 true)))
  (CallFunction|FadeOut (Utilities|Array|MakeArray (Variables|Default|GetInstanceTower) (Variables|Default|GetInstanceTower1) (Variables|Default|GetInstanceTower2))))

(fn ConstructionScript)