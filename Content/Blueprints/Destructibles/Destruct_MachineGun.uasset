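; Destructible debris actor for a machine gun, carrying low, mid and high variants of three destructible pieces.
; ConstructDestruction takes a LowMidHigh value, destroys the components of the other two variants and applies muzzle and base materials to the remaining pieces.
; It then shatters each piece with radius damage at the actor location, using a random radius and a strong impulse.
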(event Collision|EventActorBeginOverlap
  (params (OtherActor :type Actor%20Object%20Reference)))

(event EventTick
  (params (DeltaSeconds :type Float%20%28single-precision%29)))

(event EventConstructDestruction
  (params (materialToApply :type Material%20Instance%20Object%20Reference) (lowMidHigh :type Integer))
  (bind _returnvalue (Transformation|GetActorLocation))
  (bind _returnvalue_2 (Math|Random|RandomFloatinRange 1e+02 2.5e+02))
  (bind _returnvalue_3 (Transformation|GetActorLocation))
  (bind _returnvalue_4 (Math|Random|RandomFloatinRange 1e+02 2.5e+02))
  (bind _returnvalue_5 (Transformation|GetActorLocation))
  (bind _returnvalue_6 (Math|Random|RandomFloatinRange 1e+02 2.5e+02))
  (bind _destructiblehigh (Variables|Default|GetDestructibleHigh))
  (bind _destructiblehigh1 (Variables|Default|GetDestructibleHigh1))
  (bind _destructiblehigh2 (Variables|Default|GetDestructibleHigh2))
  (bind _destructiblelow (Variables|Default|GetDestructibleLow))
  (bind _destructiblelow1 (Variables|Default|GetDestructibleLow1))
  (bind _destructiblelow2 (Variables|Default|GetDestructibleLow2))
  (bind _destructiblemid (Variables|Default|GetDestructibleMid))
  (bind _destructiblemid1 (Variables|Default|GetDestructibleMid1))
  (bind _destructiblemid2 (Variables|Default|GetDestructibleMid2))
  (switch int lowMidHigh
    (:1
      (Components|DestroyComponent (Variables|Default|GetDestructibleMid))
      (Components|DestroyComponent (Variables|Default|GetDestructibleHigh))
      (Components|DestroyComponent (Variables|Default|GetDestructibleMid1))
      (Components|DestroyComponent (Variables|Default|GetDestructibleHigh2))
      (Components|DestroyComponent (Variables|Default|GetDestructibleMid2))
      (Components|DestroyComponent (Variables|Default|GetDestructibleHigh1))
      (Rendering|Material|SetMaterial _destructiblelow 0 "/Game/Materials/Glow/MachineGunMuzzle.MachineGunMuzzle")
      (Rendering|Material|SetMaterial _destructiblelow 1 "/Game/Materials/Glow/MachineGunMuzzle.MachineGunMuzzle")
      (Rendering|Material|SetMaterial _destructiblelow 3 "/Game/Materials/Glow/MachineGunMuzzle.MachineGunMuzzle")
      (Class|DestructibleComponent|ApplyRadiusDamage _destructiblelow 1e+03 _returnvalue_3 _returnvalue_4 2.5e+04 true)
      (Rendering|Material|SetMaterial _destructiblelow1 0 "/Game/Materials/Glow/MachineGunBase.MachineGunBase")
      (Rendering|Material|SetMaterial _destructiblelow1 1 "/Game/Materials/Glow/MachineGunBase.MachineGunBase")
      (Rendering|Material|SetMaterial _destructiblelow1 3 "/Game/Materials/Glow/MachineGunBase.MachineGunBase")
      (Class|DestructibleComponent|ApplyRadiusDamage _destructiblelow1 1e+03 _returnvalue_3 _returnvalue_4 2.5e+04 true)
      (Rendering|Material|SetMaterial _destructiblelow2 0 "/Game/Materials/Glow/MachineGunBase.MachineGunBase")
      (Rendering|Material|SetMaterial _destructiblelow2 1 "/Game/Materials/Glow/MachineGunBase.MachineGunBase")
      (Rendering|Material|SetMaterial _destructiblelow2 3 "/Game/Materials/Glow/MachineGunBase.MachineGunBase")
      (Class|DestructibleComponent|ApplyRadiusDamage _destructiblelow2 1e+03 _returnvalue_3 _returnvalue_4 2.5e+04 true))
    (:2
      (Components|DestroyComponent (Variables|Default|GetDestructibleLow))
      (Components|DestroyComponent (Variables|Default|GetDestructibleHigh))
      (Components|DestroyComponent (Variables|Default|GetDestructibleLow1))
      (Components|DestroyComponent (Variables|Default|GetDestructibleHigh2))
      (Components|DestroyComponent (Variables|Default|GetDestructibleLow2))
      (Components|DestroyComponent (Variables|Default|GetDestructibleHigh1))
      (Rendering|Material|SetMaterial _destructiblemid 0 "/Game/Materials/Glow/MachineGunMuzzle.MachineGunMuzzle")
      (Rendering|Material|SetMaterial _destructiblemid 1 "/Game/Materials/Glow/MachineGunMuzzle.MachineGunMuzzle")
      (Rendering|Material|SetMaterial _destructiblemid 3 "/Game/Materials/Glow/MachineGunMuzzle.MachineGunMuzzle")
      (Class|DestructibleComponent|ApplyRadiusDamage _destructiblemid 1e+03 _returnvalue_5 _returnvalue_6 2.5e+04 true)
      (Rendering|Material|SetMaterial _destructiblemid1 0 "/Game/Materials/Glow/MachineGunBase.MachineGunBase")
      (Rendering|Material|SetMaterial _destructiblemid1 1 "/Game/Materials/Glow/MachineGunBase.MachineGunBase")
      (Rendering|Material|SetMaterial _destructiblemid1 3 "/Game/Materials/Glow/MachineGunBase.MachineGunBase")
      (Class|DestructibleComponent|ApplyRadiusDamage _destructiblemid1 1e+03 _returnvalue_5 _returnvalue_6 2.5e+04 true)
      (Rendering|Material|SetMaterial _destructiblemid2 0 "/Game/Materials/Glow/MachineGunBase.MachineGunBase")
      (Rendering|Material|SetMaterial _destructiblemid2 1 "/Game/Materials/Glow/MachineGunBase.MachineGunBase")
      (Rendering|Material|SetMaterial _destructiblemid2 3 "/Game/Materials/Glow/MachineGunBase.MachineGunBase")
      (Class|DestructibleComponent|ApplyRadiusDamage _destructiblemid2 1e+03 _returnvalue_5 _returnvalue_6 2.5e+04 true))
    (:3
      (Components|DestroyComponent (Variables|Default|GetDestructibleMid))
      (Components|DestroyComponent (Variables|Default|GetDestructibleLow1))
      (Components|DestroyComponent (Variables|Default|GetDestructibleMid1))
      (Components|DestroyComponent (Variables|Default|GetDestructibleLow2))
      (Components|DestroyComponent (Variables|Default|GetDestructibleMid2))
      (Components|DestroyComponent (Variables|Default|GetDestructibleLow))
      (Rendering|Material|SetMaterial _destructiblehigh 0 "/Game/Materials/Glow/MachineGunMuzzle.MachineGunMuzzle")
      (Rendering|Material|SetMaterial _destructiblehigh 1 "/Game/Materials/Glow/MachineGunMuzzle.MachineGunMuzzle")
      (Rendering|Material|SetMaterial _destructiblehigh 3 "/Game/Materials/Glow/MachineGunMuzzle.MachineGunMuzzle")
      (Class|DestructibleComponent|ApplyRadiusDamage _destructiblehigh 1e+03 _returnvalue _returnvalue_2 2.5e+04 true)
      (Rendering|Material|SetMaterial _destructiblehigh2 0 "/Game/Materials/Glow/MachineGunBase.MachineGunBase")
      (Rendering|Material|SetMaterial _destructiblehigh2 1 "/Game/Materials/Glow/MachineGunBase.MachineGunBase")
      (Rendering|Material|SetMaterial _destructiblehigh2 3 "/Game/Materials/Glow/MachineGunBase.MachineGunBase")
      (Class|DestructibleComponent|ApplyRadiusDamage _destructiblehigh2 1e+03 _returnvalue _returnvalue_2 2.5e+04 true)
      (Rendering|Material|SetMaterial _destructiblehigh1 0 "/Game/Materials/Glow/MachineGunBase.MachineGunBase")
      (Rendering|Material|SetMaterial _destructiblehigh1 1 "/Game/Materials/Glow/MachineGunBase.MachineGunBase")
      (Rendering|Material|SetMaterial _destructiblehigh1 3 "/Game/Materials/Glow/MachineGunBase.MachineGunBase")
      (Class|DestructibleComponent|ApplyRadiusDamage _destructiblehigh1 1e+03 _returnvalue _returnvalue_2 2.5e+04 true))))

(fn ConstructionScript)