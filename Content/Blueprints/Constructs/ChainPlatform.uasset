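; Buildable platform construct that players extend into a chain by stepping on its four edge triggers.
; On authority, overlap spawns another ChainPlatform outward from that trigger, or toggles that side's WallOrder flag if spawning fails.
; End overlap applies the flags to the veil walls, enabling the ceiling only when all four are set, with HUD alerts.
; BeginPlay hides all veils and spawns a ConstructiblePad_SingleCell on top.
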(event OnComponentBeginOverlap(PlatformTrigerFwd)
  (params (OverlappedComponent :type Primitive%20Component%20Object%20Reference) (OtherActor :type Actor%20Object%20Reference) (OtherComp :type Primitive%20Component%20Object%20Reference) (OtherBodyIndex :type Integer) (bFromSweep :type Boolean) (SweepResult :type Hit%20Result%20Structure%20%28by%20ref%29))
  (bind _wallorder (Variables|Default|GetWallOrder))
  (Networking|SwitchHasAuthority
    (:Authority
      (bind _asshooter_sandbox_character (Utilities|Casting|CastToShooterSandboxCharacter OtherActor))
      (bind _spawned (CallFunction|SpawnPlatformat (Variables|Default|GetPlatformTrigerFwd) _asshooter_sandbox_character))
      (if (not _spawned)
        (Utilities|Array|SetArrayElem _wallorder 0 (not (Utilities|Array|Get(acopy) _wallorder)))))))

(event OnComponentBeginOverlap(PlatformTrigerRight)
  (params (OverlappedComponent :type Primitive%20Component%20Object%20Reference) (OtherActor :type Actor%20Object%20Reference) (OtherComp :type Primitive%20Component%20Object%20Reference) (OtherBodyIndex :type Integer) (bFromSweep :type Boolean) (SweepResult :type Hit%20Result%20Structure%20%28by%20ref%29))
  (bind _wallorder (Variables|Default|GetWallOrder))
  (Networking|SwitchHasAuthority
    (:Authority
      (bind _asshooter_sandbox_character (Utilities|Casting|CastToShooterSandboxCharacter OtherActor))
      (bind _spawned (CallFunction|SpawnPlatformat (Variables|Default|GetPlatformTrigerRight) _asshooter_sandbox_character))
      (if (not _spawned)
        (Utilities|Array|SetArrayElem _wallorder 2 (not (Utilities|Array|Get(acopy) _wallorder 2)))))))

(event OnComponentBeginOverlap(PlatformTrigerBwd)
  (params (OverlappedComponent :type Primitive%20Component%20Object%20Reference) (OtherActor :type Actor%20Object%20Reference) (OtherComp :type Primitive%20Component%20Object%20Reference) (OtherBodyIndex :type Integer) (bFromSweep :type Boolean) (SweepResult :type Hit%20Result%20Structure%20%28by%20ref%29))
  (bind _wallorder (Variables|Default|GetWallOrder))
  (Networking|SwitchHasAuthority
    (:Authority
      (bind _asshooter_sandbox_character (Utilities|Casting|CastToShooterSandboxCharacter OtherActor))
      (bind _spawned (CallFunction|SpawnPlatformat (Variables|Default|GetPlatformTrigerBwd) _asshooter_sandbox_character))
      (if (not _spawned)
        (Utilities|Array|SetArrayElem _wallorder 1 (not (Utilities|Array|Get(acopy) _wallorder 1)))))))

(event OnComponentBeginOverlap(PlatformTrigerLeft)
  (params (OverlappedComponent :type Primitive%20Component%20Object%20Reference) (OtherActor :type Actor%20Object%20Reference) (OtherComp :type Primitive%20Component%20Object%20Reference) (OtherBodyIndex :type Integer) (bFromSweep :type Boolean) (SweepResult :type Hit%20Result%20Structure%20%28by%20ref%29))
  (bind _wallorder (Variables|Default|GetWallOrder))
  (Networking|SwitchHasAuthority
    (:Authority
      (bind _asshooter_sandbox_character (Utilities|Casting|CastToShooterSandboxCharacter OtherActor))
      (bind _spawned (CallFunction|SpawnPlatformat (Variables|Default|GetPlatformTrigerLeft) _asshooter_sandbox_character))
      (if (not _spawned)
        (Utilities|Array|SetArrayElem _wallorder 3 (not (Utilities|Array|Get(acopy) _wallorder 3)))))))

(event OnComponentEndOverlap(PlatformTrigerFwd)
  (params (OverlappedComponent :type Primitive%20Component%20Object%20Reference) (OtherActor :type Actor%20Object%20Reference) (OtherComp :type Primitive%20Component%20Object%20Reference) (OtherBodyIndex :type Integer))
  (Networking|SwitchHasAuthority
    (:Authority
      (bind _asshooter_sandbox_character (Utilities|Casting|CastToShooterSandboxCharacter OtherActor))
      (CallFunction|CheckifWallBuildPending _asshooter_sandbox_character))))

(event OnComponentEndOverlap(PlatformTrigerRight)
  (params (OverlappedComponent :type Primitive%20Component%20Object%20Reference) (OtherActor :type Actor%20Object%20Reference) (OtherComp :type Primitive%20Component%20Object%20Reference) (OtherBodyIndex :type Integer))
  (Networking|SwitchHasAuthority
    (:Authority
      (bind _asshooter_sandbox_character (Utilities|Casting|CastToShooterSandboxCharacter OtherActor))
      (CallFunction|CheckifWallBuildPending _asshooter_sandbox_character))))

(event OnComponentEndOverlap(PlatformTrigerLeft)
  (params (OverlappedComponent :type Primitive%20Component%20Object%20Reference) (OtherActor :type Actor%20Object%20Reference) (OtherComp :type Primitive%20Component%20Object%20Reference) (OtherBodyIndex :type Integer))
  (Networking|SwitchHasAuthority
    (:Authority
      (bind _asshooter_sandbox_character (Utilities|Casting|CastToShooterSandboxCharacter OtherActor))
      (CallFunction|CheckifWallBuildPending _asshooter_sandbox_character))))

(event OnComponentEndOverlap(PlatformTrigerBwd)
  (params (OverlappedComponent :type Primitive%20Component%20Object%20Reference) (OtherActor :type Actor%20Object%20Reference) (OtherComp :type Primitive%20Component%20Object%20Reference) (OtherBodyIndex :type Integer))
  (Networking|SwitchHasAuthority
    (:Authority
      (bind _asshooter_sandbox_character (Utilities|Casting|CastToShooterSandboxCharacter OtherActor))
      (CallFunction|CheckifWallBuildPending _asshooter_sandbox_character))))

(event Custom|SpawnSpawnablePad
  (Networking|SwitchHasAuthority
    (:Authority
      (Game|SpawnActorfromClass "/Game/Blueprints/Constructs/ConstructiblePad_SingleCell.ConstructiblePad_SingleCell_C" (Math|Transform|MakeTransform (+ (Transformation|GetActorLocation) "0, 0,25.000000") (Transformation|GetActorRotation) "6.000000,6.000000,6.000000") "AdjustIfPossibleButDontSpawnIfColliding" 0 0))))

(event Custom|CheckIfWallBuildPending
  (params (Player :type Shooter%20Sandbox%20Character%20Object%20Reference))
  (bind _returnvalue (Pawn|GetController Player))
  (bind _returnvalue_2 (Pawn|GetController Player))
  (bind _wall_right (Variables|Default|GetWall_Right))
  (bind _wall_left (Variables|Default|GetWall_Left))
  (bind _wall_fwd (Variables|Default|GetWall_Fwd))
  (bind _wall_bwd (Variables|Default|GetWall_Bwd))
  (Variables|Default|SetCeilStatus true)
  (for (_array_element _array_index) (Variables|Default|GetWallOrder)
    (switch int _array_index
      (:0
        (Variables|Default|SetCeilStatus (and (Variables|Default|GetCeilStatus) _array_element))
        (if (Class|KismetMathLibrary|XORBoolean (Rendering|IsVisible _wall_fwd) _array_element)
          (CallFunction|DroporRaiseVeil _wall_fwd _array_element)
          (if _array_element
            (bind _asshooter_sandbox_controller (Utilities|Casting|CastToShooterSandboxController _returnvalue))
            (Class|ShooterSandboxController|ProxyforHUDAlertMessage _asshooter_sandbox_controller "Platform Veil Raised" 3)
            (else
              (bind _asshooter_sandbox_controller_2 (Utilities|Casting|CastToShooterSandboxController _returnvalue))
              (Class|ShooterSandboxController|ProxyforHUDAlertMessage _asshooter_sandbox_controller_2 "Platform Veil Lowered" 3)))))
      (:1
        (Variables|Default|SetCeilStatus (and (Variables|Default|GetCeilStatus) _array_element))
        (if (Class|KismetMathLibrary|XORBoolean (Rendering|IsVisible _wall_bwd) _array_element)
          (CallFunction|DroporRaiseVeil _wall_bwd _array_element)
          (if _array_element
            (bind _asshooter_sandbox_controller_3 (Utilities|Casting|CastToShooterSandboxController _returnvalue))
            (Class|ShooterSandboxController|ProxyforHUDAlertMessage _asshooter_sandbox_controller_3 "Platform Veil Raised" 3)
            (else
              (bind _asshooter_sandbox_controller_4 (Utilities|Casting|CastToShooterSandboxController _returnvalue))
              (Class|ShooterSandboxController|ProxyforHUDAlertMessage _asshooter_sandbox_controller_4 "Platform Veil Lowered" 3)))))
      (:2
        (Variables|Default|SetCeilStatus (and (Variables|Default|GetCeilStatus) _array_element))
        (if (Class|KismetMathLibrary|XORBoolean (Rendering|IsVisible _wall_right) _array_element)
          (CallFunction|DroporRaiseVeil _wall_right _array_element)
          (if _array_element
            (bind _asshooter_sandbox_controller_5 (Utilities|Casting|CastToShooterSandboxController _returnvalue))
            (Class|ShooterSandboxController|ProxyforHUDAlertMessage _asshooter_sandbox_controller_5 "Platform Veil Raised" 3)
            (else
              (bind _asshooter_sandbox_controller_6 (Utilities|Casting|CastToShooterSandboxController _returnvalue))
              (Class|ShooterSandboxController|ProxyforHUDAlertMessage _asshooter_sandbox_controller_6 "Platform Veil Lowered" 3)))))
      (:3
        (Variables|Default|SetCeilStatus (and (Variables|Default|GetCeilStatus) _array_element))
        (if (Class|KismetMathLibrary|XORBoolean (Rendering|IsVisible _wall_left) _array_element)
          (CallFunction|DroporRaiseVeil _wall_left _array_element)
          (if _array_element
            (bind _asshooter_sandbox_controller_7 (Utilities|Casting|CastToShooterSandboxController _returnvalue))
            (Class|ShooterSandboxController|ProxyforHUDAlertMessage _asshooter_sandbox_controller_7 "Platform Veil Raised" 3)
            (else
              (bind _asshooter_sandbox_controller_8 (Utilities|Casting|CastToShooterSandboxController _returnvalue))
              (Class|ShooterSandboxController|ProxyforHUDAlertMessage _asshooter_sandbox_controller_8 "Platform Veil Lowered" 3)))))))
  (if (Class|KismetMathLibrary|XORBoolean (Variables|Default|GetCeilStatus) (Rendering|IsVisible (Variables|Default|GetCeil)))
    (if (Variables|Default|GetCeilStatus)
      (bind _asshooter_sandbox_controller_9 (Utilities|Casting|CastToShooterSandboxController _returnvalue_2))
      (Class|ShooterSandboxController|ProxyforHUDAlertMessage _asshooter_sandbox_controller_9 "Platform Ceiling Actived" 3)
      (else
        (bind _asshooter_sandbox_controller_10 (Utilities|Casting|CastToShooterSandboxController _returnvalue_2))
        (Class|ShooterSandboxController|ProxyforHUDAlertMessage _asshooter_sandbox_controller_10 "Platform Ceiling Deactivated" 3))))
  (CallFunction|DroporRaiseVeil (Variables|Default|GetCeil) (Variables|Default|GetCeilStatus)))

(event Custom|ShutOffWalls
  (bind _returnvalue (Transformation|GetActorRotation))
  (bind _wall_bwd (Variables|Default|GetWall_Bwd))
  (bind _wall_fwd (Variables|Default|GetWall_Fwd))
  (bind _wall_right (Variables|Default|GetWall_Right))
  (bind _wall_left (Variables|Default|GetWall_Left))
  (bind _ceil (Variables|Default|GetCeil))
  (Components|Activation|SetActive _wall_bwd false false)
  (Rendering|SetVisibility _wall_bwd false false)
  (Components|Activation|SetActive _wall_fwd false false)
  (Rendering|SetVisibility _wall_fwd false false)
  (Components|Activation|SetActive _wall_right false false)
  (Rendering|SetVisibility _wall_right false false)
  (Components|Activation|SetActive _wall_left false false)
  (Rendering|SetVisibility _wall_left false false)
  (Components|Activation|SetActive _ceil false false)
  (Rendering|SetVisibility _ceil false false)
  (Utilities|FlowControl|Delay 0.5)
  (if (Math|Vector|Equal(Vector) (Math|Vector|VectorUp) (Transformation|GetActorUpVector) 5.0)
    (Transformation|SetActorRotation (Math|Rotator|MakeRotator 0.0 (.pitch _returnvalue) (.yaw _returnvalue)) true)))

(event Custom|DropOrRaiseVeil
  (params (Wall :type Static%20Mesh%20Component%20Object%20Reference) (VeilStatus :type Boolean))
  (Components|Activation|SetActive Wall VeilStatus false)
  (Rendering|SetVisibility Wall VeilStatus false))

(event EventBeginPlay
  (CallFunction|SpawnSpawnablePad)
  (CallFunction|ShutOffWalls))

(event Collision|EventActorBeginOverlap
  (params (OtherActor :type Actor%20Object%20Reference)))

(event EventTick
  (params (DeltaSeconds :type Float%20%28single-precision%29)))

(fn ConstructionScript)

(fn SpawnPlatformat
  (params (TriggeredPad :type Static%20Mesh%20Component%20Object%20Reference) (Player :type Shooter%20Sandbox%20Character%20Object%20Reference))
  (Networking|SwitchHasAuthority
    (:Authority
      (bind _returnvalue (Game|SpawnActorfromClass "ChainPlatform_C" (Math|Transform|MakeTransform (+ (Transformation|GetWorldLocation TriggeredPad) (* (Math|Vector|GetForwardVector TriggeredPad) 1050)) (Transformation|GetWorldRotation TriggeredPad)) "AdjustIfPossibleButDontSpawnIfColliding" 0 0))
      (if (Utilities|IsValid _returnvalue)
        (bind _asshooter_sandbox_controller (Utilities|Casting|CastToShooterSandboxController (Pawn|GetController Player)))
        (Class|ShooterSandboxController|ProxyforHUDAlertMessage _asshooter_sandbox_controller "Chain Platform Spawned" 3))
      (return (Utilities|IsValid _returnvalue)))))