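; Base construct actor built on a geometry collection that can be broken apart and faded out.
; The construction script disables physics and gravity and registers the child-actor anchor field as an initialization field.
; BlockifyConstruct clears that field, destroys the anchor and triggers the child force field, then starts FadeAndDestroy.
; A per-frame Delay loop lowers the dynamic material's opacity over the fade duration before calling DestroyNow.
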(event Custom|FadeAndDestroy
  (bind _returnvalue (Utilities|Time|GetWorldDeltaSeconds))
  (if (<= (Variables|Default|GetFadeOutTimePassed) (Variables|Default|GetfadeOutDuration)) :!label _label
    (bind _output_get (Variables|Default|SetFadeOutValue (/ (Variables|Default|GetFadeOutTimePassed) (Variables|Default|GetfadeOutDuration))))
    (Rendering|Material|SetScalarParameterValue (Variables|Default|GetcreatedDynamicMaterial) "Opacity" (- 1.0 _output_get) :!class /Script/Engine.MaterialInstanceDynamic)
    (Variables|Default|SetFadeOutTimePassed (+ (Variables|Default|GetFadeOutTimePassed) _returnvalue))
    (Utilities|FlowControl|Delay _returnvalue)
    (goto _label)
    (else
      (Class|BaseConstruct|DestroyNow))))

(event EventBlockifyConstruct
  (Utilities|Array|Clear (Variables|/Script/GeometryCollectionEngine.GeometryCollectionComponent|GetInitializationFields (Variables|Default|GetconstructBaseGeometry)))
  (Components|DestroyComponent (Variables|Default|GetConstructAnchorField))
  (Utilities|FlowControl|Sequence
    (:then_0
      (bind _asebase_force_field (Utilities|Casting|CastToEBaseConstructForceField (Variables|/Script/Engine.ChildActorComponent|GetChildActor (Variables|Default|GetForceField))))
      (Default|CETrigger _asebase_force_field))
    (:then_1
      (CallFunction|FadeandDestroy))))

(fn ConstructionScript
  (bind _constructbasegeometry (Variables|Default|GetconstructBaseGeometry))
  (Utilities|FlowControl|Sequence
    (:then_0
      ;[0.1637 1 0.2953] Set off Gravity
      (Physics|SetSimulatePhysics _constructbasegeometry false)
      (Physics|SetEnableGravity _constructbasegeometry false))
    (:then_1
      ;[1 0.1667 0.1667] Add Initialization Fields
      (bind _asconstruct_anchor_field (Utilities|Casting|CastToConstructAnchorField (Variables|/Script/Engine.ChildActorComponent|GetChildActor (Variables|Default|GetConstructAnchorField))))
      (Utilities|Array|Add (Variables|/Script/GeometryCollectionEngine.GeometryCollectionComponent|GetInitializationFields (Variables|Default|GetconstructBaseGeometry)) _asconstruct_anchor_field))))